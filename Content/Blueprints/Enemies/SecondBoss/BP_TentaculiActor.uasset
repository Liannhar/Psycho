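; BP_TentaculiActor is an actor among the second boss enemy assets that receives exported particle data from its Niagara component.
; On BeginPlay it moves the component to the actor's location, caches the player character and registers itself as the Niagara "CallbackCollision" object.
; Each particle in the callback data has its position printed and triggers an OnComponentBeginOverlap call.
; The actor overlap and Tick events are empty.
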(event EventBeginPlay
  (Transformation|SetWorldLocation (Variables|Default|GetNiagaraComponent) (Transformation|GetActorLocation) false false)
  (bind _asplayer_character (Utilities|Casting|CastToPlayerCharacter (Game|GetPlayerCharacter 0)))
  (Variables|Default|SetPlayer _asplayer_character)
  (Class|NiagaraComponent|SetVariableObject (Variables|Default|GetNiagaraComponent) "CallbackCollision" self))

(event Collision|EventActorBeginOverlap
  (params (OtherActor :type Actor%20Object%20Reference)))

(event EventTick
  (params (DeltaSeconds :type Float%20%28single-precision%29)))

(event EventParticleData
  (params (Data :type Array%20of%20Basic%20Particle%20Data%20Structures) (NiagaraSystem :type Niagara%20System%20Object%20Reference) (SimulationPositionOffset :type Vector%20%28by%20ref%29 :default "0, 0, 0"))
  (for _array_element Data
    (Development|PrintString (Utilities|String|ToString(Vector) (.Position (Utilities|Struct|BreakBasicParticleData _array_element))))
    (Class|TentaculiActor|OnComponentBeginOverlap)))

(fn ConstructionScript)
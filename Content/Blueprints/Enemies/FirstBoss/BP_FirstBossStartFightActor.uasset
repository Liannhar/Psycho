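; Trigger actor that starts the first boss encounter when the player character overlaps its box.
; While NeedTrigger is false, the overlap plays the boss intro montage, calls FirstBossIntro on the game instance, assigns BT_FirstBoss as the boss's behavior tree asset, and teleports the player to NewLocation.
; This graph never sets NeedTrigger, so it does not itself prevent repeat triggering.
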(event OnComponentBeginOverlap(BoxComponent)
  (params (OverlappedComponent :type Primitive%20Component%20Object%20Reference) (OtherActor :type Actor%20Object%20Reference) (OtherComp :type Primitive%20Component%20Object%20Reference) (OtherBodyIndex :type Integer) (bFromSweep :type Boolean) (SweepResult :type Hit%20Result%20Structure%20%28by%20ref%29))
  (bind _firstboss (Variables|Default|GetFirstBoss))
  (bind _asbp_player_character (Utilities|Casting|CastToBP_PlayerCharacter OtherActor))
  (Variables|Default|SetAs%20BP%20Player%20Character _asbp_player_character)
  (if (not (Variables|Default|GetNeedTrigger))
    (Animation|PlayAnimMontage _firstboss "/Game/Enemies/Fitstboss/Animations/Boss_Attack/Montages/Boss_Intro.Boss_Intro" 1.0 "None")
    (Default|FirstBossIntro (Variables|Default|GetAs%20BP%20Psycho%20Game%20Instance))
    (Variables|/Script/Psycho.BaseEnemy|SetBehaviorTreeAsset _firstboss "/Game/Blueprints/Enemies/FirstBoss/AI/BT_FirstBoss.BT_FirstBoss")
    (Transformation|SetActorLocation (Variables|Default|GetAs%20BP%20Player%20Character) (Variables|Default|GetNew%20Location) false false)))

(event EventBeginPlay
  (Variables|Default|SetAs%20BP%20Psycho%20Game%20Instance (.AsBP%20Psycho%20Game%20Instance (Utilities|Casting|CastToBP_PsychoGameInstance (Game|GetGameInstance)))))

(event EventTick
  (params (DeltaSeconds :type Float%20%28single-precision%29)))

(fn ConstructionScript)
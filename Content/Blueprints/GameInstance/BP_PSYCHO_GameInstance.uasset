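; BP_PSYCHO_GameInstance is the game instance that holds shared events for the HUD and for level-wide door control.
; It creates the WB_HUD widget, adds it to the viewport and sets game-only input.
; Door events gather every BP_Door_Base actor and open or close them all, printing debug text.
; A block-interaction X on the HUD is shown through render opacity, then hidden after a short retriggerable delay.
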(event Custom|Create_Widget
  ;[1 1 1] Create Widget
  (CallFunction|CreateWidgets))

(event Custom|Show%20Block
  ;[1 1 1] Show/Hide X widget
  (Widget|SetRenderOpacity (Variables|/Game/Blueprints/InteractionSystem/WIdgets/WB_Block_Interaction.WB_Block_Interaction_C|GetX (Variables|/Game/Blueprints/HUD/WB_HUD.WB_HUD_C|GetWB_Block_Interaction (Variables|Default|GetWB_HUD))) 1.0)
  (Utilities|FlowControl|RetriggerableDelay 2.0)
  (CallFunction|HideBlock))

(event Custom|Hide_Block
  ;[1 1 1] Show/Hide X widget
  (Widget|SetRenderOpacity (Variables|/Game/Blueprints/InteractionSystem/WIdgets/WB_Block_Interaction.WB_Block_Interaction_C|GetX (Variables|/Game/Blueprints/HUD/WB_HUD.WB_HUD_C|GetWB_Block_Interaction (Variables|Default|GetWB_HUD))) 0.0))

(event Custom|Get_close
  ;[1 1 1] Close/Open Door Event
  (bind _outactors (Actor|GetAllActorsOfClass "/Game/Blueprints/Doors/BP_Door_Base.BP_Door_Base_C"))
  (bind _output_get (Variables|Default|Setdoors _outactors))
  (bind _result (Math|Integer|DecrementInt (Utilities|Array|Length _output_get))
    (:%20%20
      (for _index (range 0 _result)
        (Default|Close (Utilities|Array|Get(acopy) _output_get _index))
        (Development|PrintString "close")))))

(event Custom|Get_Open
  ;[1 1 1] Close/Open Door Event
  (bind _outactors (Actor|GetAllActorsOfClass "/Game/Blueprints/Doors/BP_Door_Base.BP_Door_Base_C"))
  (bind _output_get (Variables|Default|Setdoors _outactors))
  (bind _result (Math|Integer|DecrementInt (Utilities|Array|Length _output_get))
    (:%20%20
      (for _index (range 0 _result)
        (Default|Open (Utilities|Array|Get(acopy) _output_get _index))
        (Development|PrintString "Open")))))

(fn CreateWidgets
  (bind _returnvalue (UserInterface|CreateWidget "/Game/Blueprints/HUD/WB_HUD.WB_HUD_C"))
  (bind _output_get (Variables|Default|SetWB_HUD _returnvalue))
  (UserInterface|Viewport|AddtoViewport _output_get 0)
  (Input|SetInputModeGameOnly (Game|GetPlayerController 0)))
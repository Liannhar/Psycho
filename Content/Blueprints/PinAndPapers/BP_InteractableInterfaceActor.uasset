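; BP_InteractableInterfaceActor is a placeable interactable, either a letter or a pin code, that opens an on-screen UI when a character interacts with it.
; The construction script picks the static mesh from InterfaceType.
; Interaction creates WBP_InteractableInterface, passing it the type, door to open, correct code and letter text.
; It then ignores move and look input, switches to UI-only input and shows the mouse cursor.
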(event EventInteraction
  (params (Char_Ref :type BP%20Player%20Character%20Object%20Reference))
  (bind _returnvalue (Game|GetPlayerController 0))
  (bind _asplayer_controller (Utilities|Casting|CastToPlayerController (Pawn|GetController Char_Ref)))
  (bind _returnvalue_2 (UserInterface|CreateWidget "/Game/Blueprints/PinAndPapers/WBP_InteractableInterface.WBP_InteractableInterface_C" _asplayer_controller))
  (Default|SetupWidget _returnvalue_2 (Variables|Interface|GetInterfaceType) (Variables|PinCode|GetDoorToOpen) (Variables|PinCode|GetCorrectCode) (Variables|Letter|GetLetterText))
  (UserInterface|Viewport|AddtoViewport _returnvalue_2 0)
  (Input|SetIgnoreMoveInput _returnvalue true)
  (Input|SetIgnoreLookInput _returnvalue true)
  (Input|SetInputModeUIOnly _returnvalue 0 "DoNotLock")
  (Variables|/Script/Engine.PlayerController|SetbShowMouseCursor _returnvalue true))

(fn ConstructionScript
  (switch Utilities|FlowControl|Switch|SwitchonENum_InteractableInterface (Variables|Interface|GetInterfaceType)
    (:NewEnumerator0
      (Components|StaticMesh|SetStaticMesh (Variables|Default|GetStaticMesh) (Variables|Letter|GetSM_Letter)))
    (:NewEnumerator1
      (Components|StaticMesh|SetStaticMesh (Variables|Default|GetStaticMesh) (Variables|PinCode|GetSM_PinCode)))))
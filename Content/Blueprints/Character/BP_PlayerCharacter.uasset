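; Player character Blueprint that has the game instance create a widget on BeginPlay and handles interaction input.
; IA_Interact runs a debug-drawn visibility trace from the actor along the camera's forward vector and sends InteractionMessage to the hit actor.
; Canceling the input clears HoldTimer, which is not set in this graph, and activates character movement.
; Keys 1 and 2 call GetOpen and GetClose on the game instance.
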(event Custom|ClearTimer
  (Utilities|Time|ClearandInvalidateTimerbyHandle (Variables|Default|GetHoldTimer))
  (Components|Activation|Activate (Variables|Character|GetCharacterMovement) false))

(event Input|EnhancedActionEvents|EnhancedInputActionIA_Interact
  (params (ActionValue :type Boolean) (ElapsedSeconds :type Float%20%28double-precision%29) (TriggeredSeconds :type Float%20%28double-precision%29) (InputAction :type Input%20Action%20Object%20Reference :default "/Game/Blueprints/Inputs/Default/IA_Interact.IA_Interact"))
  (bind _returnvalue (Transformation|GetActorLocation))
  (:Triggered
    (bind (_outhit _returnvalue_2) (Collision|LineTraceByChannel _returnvalue (+ _returnvalue (* (Math|Vector|GetForwardVector (Variables|Default|GetFollowCamera)) 2e+02)) "TraceTypeQuery1" false 0 "ForDuration"))
    (if _returnvalue_2
      (Class|BPIInteraction|Interaction(Message) (.HitActor (Collision|BreakHitResult _outhit)) self)))
  (:Canceled
    (CallFunction|ClearTimer)))

(event EventBeginPlay
  (bind _output_get (Variables|Default|SetGameInst (.AsBP%20PSYCHO%20Game%20Instance (Utilities|Casting|CastToBP_PSYCHO_GameInstance (Game|GetGameInstance)))))
  (Default|CreateWidget _output_get))

(event Input|KeyboardEvents|1
  (params (Key :type Key%20Structure :default "None"))
  (:Pressed
    (Default|GetOpen (Variables|Default|GetGameInst))))

(event Input|KeyboardEvents|2
  (params (Key :type Key%20Structure :default "None"))
  (:Pressed
    (Default|GetClose (Variables|Default|GetGameInst))))

(fn ConstructionScript)
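; Interactable single door Blueprint that swings open or closed when a character uses a press-type interaction.
; Open and Close events toggle CanInteract and a gate that guards the interaction.
; OpenDoor plays or reverses a timeline rotating RotateScene up to 90 degrees, choosing the swing side from a DoorRotation dot product, and activates the character's movement.
; Hold-timer and block-display logic exist but are unconnected.
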(event Custom|Open
  (Variables|Default|SetCan_Interact true)
  (Utilities|FlowControl|Gate false) ; enters at Open
)

(event Custom|Open%20Door
  ;[1 1 1] Open Door
  (Utilities|FlowControl|Sequence
    (:then_0
      (if (Variables|Default|GetDoor_Open)
        (Variables|Default|SetDot_Product (CallFunction|DoorRotation))
        (bind _alpha (Timeline|Timeline_0 Play)
          (:Update
            (Transformation|SetRelativeRotation (Variables|Default|GetRotate_Scene) (Math|Rotator|MakeRotator 0.0 0.0 (Math|Float|Lerp 0.0 (Math|Float|SelectFloat 9e+01 -9e+01 (>= (Variables|Default|GetDot_Product) 0.0)) _alpha)) false false)
            (Variables|Default|SetDoor_Open (not (> _alpha 0.0)))))
        (else
          (Timeline|Timeline_0 Reverse))))
    (:then_1
      (Components|Activation|Activate (Variables|/Script/Engine.Character|GetCharacterMovement (Variables|Default|GetChar%20Ref)) false))))

(event Custom|Close
  (Variables|Default|SetCan_Interact false)
  (Utilities|FlowControl|Gate false) ; enters at Close
)

(event EventInteraction
  (params (Char_Ref :type BP%20Player%20Character%20Object%20Reference))
  (Variables|Default|SetChar%20Ref Char_Ref)
  (if (not (not (Variables|Default|GetCan_Interact)))
    (Utilities|FlowControl|Gate false
      (:Exit
        ;[1 1 1] Choose press/hold
        (switch Utilities|FlowControl|Switch|SwitchonEnum_Interact (.Type (Utilities|Struct|BreakStructure_Interact (Variables|Default|GetData)))
          (:NewEnumerator0
            (CallFunction|OpenDoor)))))))

(fn ConstructionScript
  (|CallParentFunction))
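; BP_Door_Base is a base door Blueprint that supplies shared setup and empty Open, Close and OpenDoor events.
; On BeginPlay it allows interaction only when neither a pin code nor a key is needed.
; It also binds DelegateOpen, an empty event here, to StartFightActor when that actor is valid.
; DoorRotation returns the dot product of the character-to-door direction and the door's forward vector, indicating the character's side.
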(event Custom|DelegateOpen
  (params (IsOpen :type Boolean)))

(event Custom|Open%20Door)

(event Custom|Open)

(event Custom|Close)

(event EventBeginPlay
  (bind _startfightactor (Variables|Default|GetStartFightActor))
  (Variables|Default|SetCan_Interact (not (or (Variables|Default|GetNeedPinCode) (Variables|Default|GetNeedKey))))
  (Utilities|IsValid _startfightactor
    (:Is%20Valid
      (EventDispatchers|BindEventtoOpenDoor _startfightactor (delegate Custom|DelegateOpen)))))

(fn ConstructionScript)

(fn DoorRotation
  (bind _defaultsceneroot (Variables|Default|GetDefaultSceneRoot))
  (return (Math|Vector|DotProduct (Math|Vector|Normalize (- (Transformation|GetWorldLocation _defaultsceneroot) (Transformation|GetActorLocation (Variables|Default|GetChar%20Ref)))) (Math|Vector|GetForwardVector _defaultsceneroot))))
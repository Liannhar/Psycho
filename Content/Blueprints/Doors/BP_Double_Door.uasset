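; Interactable double door that swings both leaves open or shut on a press or timed hold, or shows a block message when locked.
; Hold mode freezes character movement until a timer fires the toggle.
; A timeline rotates the leaves in mirror, picking swing side from a dot product and reversing to close.
; A delegate event sets the lock after a short delay, closing an open door when locking and switching the interaction gate.
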(event Custom|Open%20Door
  ;[1 1 1] Open Door
  (Utilities|FlowControl|Sequence
    (:then_0
      (if (Variables|Default|GetDoor_Open)
        (Variables|Default|SetDot_Product (CallFunction|DoorRotation))
        (bind _alpha (Timeline|Timeline_0 Play)
          (:Update
            (Transformation|SetRelativeRotation (Variables|Default|GetRotate_Scene) (Math|Rotator|MakeRotator 0.0 0.0 (Math|Float|Lerp 0.0 (Math|Float|SelectFloat 9e+01 -9e+01 (>= (Variables|Default|GetDot_Product) 0.0)) _alpha)) false false)
            (Transformation|SetRelativeRotation (Variables|Default|GetRotate_Scene_2) (Math|Rotator|MakeRotator 0.0 0.0 (* (Math|Float|Lerp 0.0 (Math|Float|SelectFloat 9e+01 -9e+01 (>= (Variables|Default|GetDot_Product) 0.0)) _alpha) -1.0)) false false)
            (Variables|Default|SetDoor_Open (not (> _alpha 0.0)))))
        (else
          (Timeline|Timeline_0 Reverse))))
    (:then_1
      (Components|Activation|Activate (Variables|/Script/Engine.Character|GetCharacterMovement (Variables|Default|GetChar%20Ref)) false))))

(event EventDelegateOpen
  (params (IsOpen :type Boolean))
  (bind _data (Variables|Default|GetData))
  (bind _char_ref (Variables|Default|GetChar%20Ref))
  (bind _char_ref_2 (Variables|Default|GetChar%20Ref))
  (bind (_name _type _duration) (Utilities|Struct|BreakStructure_Interact _data))
  (Utilities|FlowControl|Delay 0.5)
  (bind _output_get (Variables|Default|SetCanInteract IsOpen))
  (if (and (not _output_get) (not (Variables|Default|GetDoor_Open)))
    (CallFunction|OpenDoor))
  (if _output_get
    (Utilities|FlowControl|Gate false) ; enters at Open
    (else
      (Utilities|FlowControl|Gate false) ; enters at Close
    )))

(event EventInteraction
  (params (Char_Ref :type BP%20Player%20Character%20Object%20Reference))
  (bind _data (Variables|Default|GetData))
  (bind (_name _type _duration) (Utilities|Struct|BreakStructure_Interact _data))
  (Variables|Default|SetChar%20Ref Char_Ref)
  (if (not (Variables|Default|GetCanInteract))
    (Default|ShowBlock (Variables|/Game/Blueprints/Character/BP_PlayerCharacter.BP_PlayerCharacter_C|GetGameInst (Variables|Default|GetChar%20Ref)))
    (else
      (Utilities|FlowControl|Gate false
        (:Exit
          ;[1 1 1] Choose press/hold
          (switch Utilities|FlowControl|Switch|SwitchonEnum_Interact _type
            (:NewEnumerator0
              (CallFunction|OpenDoor))
            (:NewEnumerator1
              ;[1 1 1] Set timer to open
              (Default|ClearTimer (Variables|Default|GetChar%20Ref))
              (bind _output_get (Variables|/Game/Blueprints/Character/BP_PlayerCharacter.BP_PlayerCharacter_C|SetDuration (Variables|Default|GetChar%20Ref) _duration))
              (bind _returnvalue (Utilities|Time|SetTimerbyEvent (delegate Custom|Open%20Door) _output_get))
              (Variables|/Game/Blueprints/Character/BP_PlayerCharacter.BP_PlayerCharacter_C|SetHoldTimer (Variables|Default|GetChar%20Ref) _returnvalue)
              (Components|Activation|Deactivate (Variables|/Script/Engine.Character|GetCharacterMovement (Variables|Default|GetChar%20Ref))))))))))

(fn ConstructionScript
  (|CallParentFunction))
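; Base weapon actor that a character picks up or swaps to by interacting with it.
; Its Interaction event passes the actor and its class to ChangeWeapon on the character's WeaponComponent, which handles the swap.
; An empty custom event and an unconnected chain that copies the mesh onto the character and destroys the actor never take effect.
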(event Custom|CustomEvent
  (params (Char_Ref :type BP%20Player%20Character%20Object%20Reference)))

(event EventBeginPlay)

(event Collision|EventActorBeginOverlap
  (params (OtherActor :type Actor%20Object%20Reference)))

(event EventTick
  (params (DeltaSeconds :type Float%20%28single-precision%29)))

(event EventInteraction
  (params (Char_Ref :type BP%20Player%20Character%20Object%20Reference))
  (Class|WeaponComponent|ChangeWeapon (Variables|/Script/Psycho.BaseCharacter|GetWeaponComponent Char_Ref) self (Utilities|GetClass self)))

(fn ConstructionScript)
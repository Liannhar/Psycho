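; Psycho character Blueprint that runs a four-hit melee combo on left mouse clicks.
; NormalAttack picks one of four attack subgraphs by AttackCounter, each playing its montage and setting the next counter, with the last wrapping to zero.
; Clicks during an attack buffer SaveAttack and start a retriggerable timeout to ComboEnd.
; NormalAttackCombo consumes the buffer to chain the next hit, or ends the combo, clearing Attacking after a delay.
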(event Custom|Normal%20Attack
  (if (Variables|Default|GetAttacking?)
    (Variables|Default|SetSave%20Attack? true)
    (Utilities|FlowControl|RetriggerableDelay 2.0)
    (CallFunction|ComboEnd)
    (else
      (switch int (Variables|Default|GetAttack%20Counter)
        (:0
          (|1Attack))
        (:1
          (|2Attack))
        (:2
          (|3Attack))
        (:3
          (|4Attack))))))

(event Custom|Normal%20Attack%20Combo
  (if (Variables|Default|GetSave%20Attack?)
    (Variables|Default|SetSave%20Attack? false)
    (switch int (Variables|Default|GetAttack%20Counter)
      (:0
        (|1Attack))
      (:1
        (|2Attack))
      (:2
        (|3Attack))
      (:3
        (|4Attack)))
    (else
      (CallFunction|ComboEnd))))

(event Custom|Combo%20End
  ;[1 1 1] Combo End
  (Variables|Default|SetAttack%20Counter 0)
  (Utilities|FlowControl|Delay 1.0)
  (Variables|Default|SetAttacking? false))

(event Input|MouseEvents|LeftMouseButton
  (params (Key :type Key%20Structure :default "None"))
  (:Pressed
    (CallFunction|NormalAttack)))

(fn ConstructionScript)
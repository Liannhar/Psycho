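; BP_Track is a short-lived afterimage actor that shows a frozen copy of player character 0's current pose.
; On BeginPlay its PoseableMesh takes the player's skeletal mesh and pose, with M_FirstBossLine applied to selected material slots.
; It randomizes the materials' Random parameter, drives Alpha with a timeline, and destroys itself when the timeline finishes.
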(event EventBeginPlay
  (bind _returnvalue (Game|GetPlayerCharacter 0))
  (bind _poseablemesh (Variables|Default|GetPoseableMesh))
  (bind _poseablemesh_2 (Variables|Default|GetPoseableMesh))
  (bind _mesh (Variables|/Script/Engine.Character|GetMesh _returnvalue))
  (Class|SkinnedMeshComponent|SetSkeletalMesh _poseablemesh_2 (Variables|/Script/Engine.SkinnedMeshComponent|GetSkeletalMesh _mesh) true)
  (Rendering|Material|SetMaterial _poseablemesh_2 1 "/Game/Enemies/Fitstboss/Niagara/Materials/M_FirstBossLine.M_FirstBossLine")
  (Rendering|Material|SetMaterial _poseablemesh_2 2 "/Game/Enemies/Fitstboss/Niagara/Materials/M_FirstBossLine.M_FirstBossLine")
  (Rendering|Material|SetMaterial _poseablemesh_2 3 "/Game/Enemies/Fitstboss/Niagara/Materials/M_FirstBossLine.M_FirstBossLine")
  (Rendering|Material|SetMaterial _poseablemesh_2 4 "/Game/Enemies/Fitstboss/Niagara/Materials/M_FirstBossLine.M_FirstBossLine")
  (Rendering|Material|SetMaterial _poseablemesh_2 18 "/Game/Enemies/Fitstboss/Niagara/Materials/M_FirstBossLine.M_FirstBossLine")
  (Rendering|Material|SetScalarParameterValueonMaterials _poseablemesh "Random" (Math|Random|RandomFloat))
  (Class|PoseableMeshComponent|CopyPosefromSkeletalComponent _poseablemesh _mesh)
  (bind _newtrack_0 (Timeline|Timeline_0 PlayFromStart)
    (:Update
      (Rendering|Material|SetScalarParameterValueonMaterials _poseablemesh "Alpha" _newtrack_0))
    (:Finished
      (Actor|DestroyActor))))

(event Collision|EventActorBeginOverlap
  (params (OtherActor :type Actor%20Object%20Reference)))

(event EventTick
  (params (DeltaSeconds :type Float%20%28single-precision%29)))

(fn ConstructionScript)